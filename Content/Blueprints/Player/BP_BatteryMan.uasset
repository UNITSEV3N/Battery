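; BP_BatteryMan is the player Blueprint that handles startup display settings and pause menu toggling.
; On BeginPlay it clears the Player reference on player 0's BatteryMan character, then enables and applies VSync.
; The Pause input creates the PAUSE_Menu widget on first use and caches it.
; Each press then toggles the menu, game pause, mouse cursor and input mode together.
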(event `self.ReceiveBeginPlay`
  ;[1 1 1] Comment
  (bind _asbp_battery_man (cast `/Game/Blueprints/Player/BP_BatteryMan` (`GameplayStatics.GetPlayerCharacter` 0)))
  (set `/Game/Blueprints/Player/BP_BatteryMan.Player` null _asbp_battery_man)
  (bind _returnvalue (`GameUserSettings.GetGameUserSettings`))
  (`GameUserSettings.SetVSyncEnabled` _returnvalue true)
  (`GameUserSettings.ApplySettings` _returnvalue true))

(event `InputAction|Pause`
  (params (Key :type "Key Structure"))
  (bind _returnvalue (`GameplayStatics.GetPlayerController` 0))
  (bind _pausemenu_ref (`self.PauseMenu_ref`))
  ;[1 1 1] Pause/Unnpause Game
  (:`Pressed`
    (`/Engine/EditorBlueprintResources/StandardMacros.IsValid` (`self.PauseMenu_ref`)
      (:`Is Valid`
        _)
      (:`Is Not Valid`
        (bind _returnvalue_2 (`|CreateWidget` "/Game/HUD/PAUSE_Menu.PAUSE_Menu_C"))
        (set `self.PauseMenu_ref` _returnvalue_2)))
    (if (`GameplayStatics.IsGamePaused`)
      (`Widget.RemoveFromParent` _pausemenu_ref)
      (set `PlayerController.bShowMouseCursor` false _returnvalue)
      (`GameplayStatics.SetGamePaused` false)
      (`WidgetBlueprintLibrary.SetInputMode_GameOnly` _returnvalue)
      (else
        (`UserWidget.AddToViewport` _pausemenu_ref 0)
        (set `PlayerController.bShowMouseCursor` true _returnvalue)
        (`GameplayStatics.SetGamePaused` true)
        (`WidgetBlueprintLibrary.SetInputMode_GameAndUIEx` _returnvalue _pausemenu_ref "DoNotLock" false)))))

(fn `UserConstructionScript`)